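; Blueprint function library that handles piece interactions, with Move as the only implemented action.
; InterAct switches on the action type, spends action points and writes the cursor location to the piece's blackboard as TargetLocation.
; ConsumeActionPoint subtracts a fixed per-action cost from the piece's CurrentActionPoint, without checking whether enough points remain.
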(fn InterAct
  (params (Piece :type BP%20TTS%20Piece%20Base%20Object%20Reference) (InterActObj :type Actor%20Object%20Reference) (InterActWhat :type E_InterAct%20Enum :default "NewEnumerator0") (CursorLocation :type Vector))
  (switch Utilities|FlowControl|Switch|SwitchonE_InterAct InterActWhat
    (:NewEnumerator0
      (CallFunction|ConsumeActionPoint Piece InterActWhat)
      (AI|Components|Blackboard|SetValueasVector (AI|GetBlackboard Piece) (Utilities|Name|MakeLiteralName "TargetLocation") CursorLocation))))

(fn ConsumeActionPoint
  (params (Piece :type BP%20TTS%20Piece%20Base%20Object%20Reference) (InterAct :type E_InterAct%20Enum :default "NewEnumerator0"))
  (switch Utilities|FlowControl|Switch|SwitchonE_InterAct InterAct
    (:NewEnumerator0
      (bind _output_get (LocalVariables|SetUseActionPoint 1.0))
      (Variables|/Game/BluePrint/Piece/BP_TTSPieceBase.BP_TTSPieceBase_C|SetCurrentActionPoint Piece (- (Variables|/Game/BluePrint/Piece/BP_TTSPieceBase.BP_TTSPieceBase_C|GetCurrentActionPoint Piece) _output_get)))))