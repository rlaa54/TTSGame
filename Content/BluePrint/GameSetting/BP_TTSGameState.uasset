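; Game state that runs the in-game clock and day counter.
; BeginPlay seeds GameTime from the starting hour, minute and second, and GameSpeed from its default.
; Tick adds DeltaSeconds divided by GameSpeed, wraps at 24 hours into GameDay, and derives GameClock.
; UpdateGameSpeed multiplies the current GameSpeed, so changes compound and higher values slow time, then calls CallGameSpeedControll with the result.
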(event EventBeginPlay
  ;[1 1 1] Game speed and time init
  (Utilities|FlowControl|Sequence
    (:then_0
      (Variables|GameClock|SetGameTime (Math|Conversions|ToFloat(Integer) (+ (Variables|GameClock|GetGameHour) (/ (Variables|GameClock|GetGameMinute) 60) (/ (Variables|GameClock|GetGameSecond) 3600))))
      (Variables|GameClock|SetGameClock (Utilities|Array|MakeArray (Variables|GameClock|GetGameHour) (Variables|GameClock|GetGameMinute) (Variables|GameClock|GetGameSecond))))
    (:then_1
      (Variables|GameSpeed|SetGameSpeed (Variables|GameSpeed|GetDefaultGameSpeed)))))

(event EventTick
  (params (DeltaSeconds :type Float%20%28single-precision%29))
  ;[1 1 1] game time flow
  (bind _output_get (Variables|GameClock|SetGameTime (.GameTimer (CallFunction|SetGameTime DeltaSeconds (Variables|GameSpeed|GetGameSpeed) (Variables|GameClock|GetGameTime)))))
  (CallFunction|SetGameClock self _output_get)
  (bind _output_get_2 (Variables|GameDay|SetDayCounter (.DayCount (CallFunction|SetGameTime DeltaSeconds (Variables|GameSpeed|GetGameSpeed) (Variables|GameClock|GetGameTime)))))
  (Variables|GameDay|SetGameDay (+ _output_get_2 (Variables|GameDay|GetGameDay))))

(event EventUpdateGameSpeed
  (params (SpeedMultiplier :type Float%20%28single-precision%29))
  ;[1 1 1] when game speed change
  (bind _output_get (Variables|GameSpeed|SetGameSpeed (* SpeedMultiplier (Variables|GameSpeed|GetGameSpeed))))
  (Default|CallGameSpeedControll _output_get))

(fn ConstructionScript)

(fn SetGameTime
  (params (DeltaTIme :type Float%20%28single-precision%29) (GameSpeed :type Float%20%28single-precision%29) (SetGameTime :type Float%20%28single-precision%29))
  (bind _returnvalue (/ DeltaTIme GameSpeed))
  (bind _returnvalue_2 (+ _returnvalue SetGameTime))
  (bind (_remainder _returnvalue_3) (Math|Float|Division(WholeandRemainder) _returnvalue_2 24.0))
  (return _remainder _returnvalue_3))

(fn SetGameClock
  (params (GameTime :type Float%20%28single-precision%29))
  (bind _returnvalue (* GameTime 3.6e+03))
  (bind (_remainder _returnvalue_2) (Math|Float|Division(WholeandRemainder) _returnvalue 6e+01))
  (bind _returnvalue_3 (Math|Conversions|ToFloat(Integer) _returnvalue_2))
  (bind (_remainder_2 _returnvalue_4) (Math|Float|Division(WholeandRemainder) _returnvalue_3 6e+01))
  (Variables|GameClock|SetGameSecond (Math|Float|Truncate _remainder))
  (Variables|GameClock|SetGameMinute (Math|Float|Truncate _remainder_2))
  (Variables|GameClock|SetGameHour (Math|Float|Truncate (.Remainder (Math|Float|Division(WholeandRemainder) (Math|Conversions|ToFloat(Integer) _returnvalue_4) 24.0))))
  (Variables|GameClock|SetGameClock (Utilities|Array|MakeArray (Variables|GameClock|GetGameHour) (Variables|GameClock|GetGameMinute) (Variables|GameClock|GetGameSecond)))
  (return))