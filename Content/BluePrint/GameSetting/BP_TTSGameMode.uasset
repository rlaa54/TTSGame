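; Game mode for the TTS piece-based game that populates the level with pieces when play begins.
; BeginPlay gathers every BP_TTSPieceSpawnBox and spawns a BP_TTSPieceBase at each box's transform.
; TurnOn is an empty event, and unconnected draft nodes sketch an initiative system that adds a random 1–20 roll to each active piece's initiating speed and begins reordering by turn speed.
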(event Custom|TurnOn)

(event EventBeginPlay
  (Utilities|FlowControl|Sequence
    (:then_0
      (bind _outactors (Actor|GetAllActorsOfClass "/Game/BluePrint/Piece/BP_TTSPieceSpawnBox.BP_TTSPieceSpawnBox_C"))
      (Variables|Reference|SetSpawnBoxRef _outactors))
    (:then_1
      (for _array_element (Variables|Reference|GetSpawnBoxRef)
        (Game|SpawnActorfromClass "/Game/BluePrint/Piece/BP_TTSPieceBase.BP_TTSPieceBase_C" (Transformation|GetActorTransform _array_element) "Undefined" 0 0)))))

(fn ConstructionScript)