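; Player controller for a TTS game that handles piece selection, piece commands and control of the TTS camera pawn.
; Left-click selects the piece under the cursor, clearing the previous selection.
; Right-click release with a piece selected opens an interact menu at the mouse, sets the piece's destination and triggers its action component, unless panning.
; Input moves, rotates and spring-arm-zooms the camera, with a gate and hold timer separating pans from clicks.
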(event EventBeginPlay
  ;[1 1 1] cam init
  (Utilities|FlowControl|Sequence
    (:then_0
      (Utilities|ReferenceCast)
      (Variables|CameraSetting|SetZoomDefault (Variables|/Script/Engine.SpringArmComponent|GetTargetArmLength (Variables|/Game/BluePrint/Camera/BP_TTSCameraPawn.BP_TTSCameraPawn_C|GetSpringArm (Variables|Reference|GetTTSCameraRef)))))
    (:then_1
      (Variables|Default|SetbEnableMouseOverEvents true))))

(event Input|ActionEvents|InputActionZoomIn
  (params (Key :type Key%20Structure :default "None"))
  (bind _ttscameraref (Variables|Reference|GetTTSCameraRef))
  (bind _springarm (Variables|/Game/BluePrint/Camera/BP_TTSCameraPawn.BP_TTSCameraPawn_C|GetSpringArm _ttscameraref))
  ;[1 1 1] cam zoom
  (:Pressed
    (Variables|/Script/Engine.SpringArmComponent|SetTargetArmLength _springarm (Math|Float|Clamp(Float) (- (Variables|/Script/Engine.SpringArmComponent|GetTargetArmLength _springarm) (Variables|CameraSetting|GetZoomSpeed)) (Variables|CameraSetting|GetZoomInMax) (Variables|CameraSetting|GetZoomOutMax)))))

(event Input|ActionEvents|InputActionZoomOut
  (params (Key :type Key%20Structure :default "None"))
  (bind _ttscameraref (Variables|Reference|GetTTSCameraRef))
  (bind _springarm (Variables|/Game/BluePrint/Camera/BP_TTSCameraPawn.BP_TTSCameraPawn_C|GetSpringArm _ttscameraref))
  ;[1 1 1] cam zoom
  (:Pressed
    (Variables|/Script/Engine.SpringArmComponent|SetTargetArmLength _springarm (Math|Float|Clamp(Float) (+ (Variables|CameraSetting|GetZoomSpeed) (Variables|/Script/Engine.SpringArmComponent|GetTargetArmLength _springarm)) (Variables|CameraSetting|GetZoomInMax) (Variables|CameraSetting|GetZoomOutMax)))))

(event Input|ActionEvents|InputActionZoomReset
  (params (Key :type Key%20Structure :default "None"))
  ;[1 1 1] cam zoom
  (:Pressed
    (Variables|/Script/Engine.SpringArmComponent|SetTargetArmLength (Variables|/Game/BluePrint/Camera/BP_TTSCameraPawn.BP_TTSCameraPawn_C|GetSpringArm (Variables|Reference|GetTTSCameraRef)) (Variables|CameraSetting|GetZoomDefault))))

(event Input|ActionEvents|InputActionPan
  (params (Key :type Key%20Structure :default "None"))
  (bind _panspeed (Variables|CameraSetting|GetPanSpeed))
  (bind _ttscameraref (Variables|Reference|GetTTSCameraRef))
  (bind _returnvalue (Transformation|GetActorRotation _ttscameraref))
  (bind (_roll _pitch _yaw) (Math|Rotator|BreakRotator _returnvalue))
  ;[1 1 1] cam panning
  (:Pressed
    (Utilities|FlowControl|Gate true) ; enters at Open
  )
  (:Released
    (Variables|Default|SetTimer 0.0)
    (Utilities|FlowControl|Gate true) ; enters at Close
  ))

(event Input|ActionEvents|InputActionPanReset
  (params (Key :type Key%20Structure :default "None"))
  ;[1 1 1] cam pan reset
  (:Pressed
    (Transformation|SetActorRotation (Variables|Reference|GetTTSCameraRef) (Math|Rotator|MakeRotator 0.0 0.0 0.0))))

(event Input|AxisEvents|InputAxisMoveForward
  (params (AxisValue :type Float%20%28single-precision%29))
  (bind _ttscameraref (Variables|Reference|GetTTSCameraRef))
  (bind _returnvalue (Transformation|GetActorForwardVector _ttscameraref))
  (bind _returnvalue_2 (Transformation|GetActorRightVector _ttscameraref))
  (bind (_x _y) (Math|Vector|BreakVector _returnvalue))
  (bind (_x_2 _y_2) (Math|Vector|BreakVector _returnvalue_2))
  ;[1 1 1] cam move
  (Transformation|SetActorLocation _ttscameraref (+ (Transformation|GetActorLocation _ttscameraref) (* (Math|Vector|MakeVector _x _y 0.0) (* AxisValue (Variables|CameraSetting|GetCameraSpeed))) (* (Math|Vector|MakeVector _x_2 _y_2 0.0) (* (stale Input|AxisEvents|InputAxisMoveRight AxisValue) (Variables|CameraSetting|GetCameraSpeed)))) true false))

(event Input|AxisEvents|InputAxisMoveRight
  (params (AxisValue :type Float%20%28single-precision%29))
  (bind _ttscameraref (Variables|Reference|GetTTSCameraRef))
  (bind _returnvalue (Transformation|GetActorForwardVector _ttscameraref))
  (bind _returnvalue_2 (Transformation|GetActorRightVector _ttscameraref))
  (bind (_x _y) (Math|Vector|BreakVector _returnvalue))
  (bind (_x_2 _y_2) (Math|Vector|BreakVector _returnvalue_2))
  ;[1 1 1] cam move
  (Transformation|SetActorLocation _ttscameraref (+ (Transformation|GetActorLocation _ttscameraref) (* (Math|Vector|MakeVector _x _y 0.0) (* (stale Input|AxisEvents|InputAxisMoveForward AxisValue) (Variables|CameraSetting|GetCameraSpeed))) (* (Math|Vector|MakeVector _x_2 _y_2 0.0) (* AxisValue (Variables|CameraSetting|GetCameraSpeed)))) true false))

(event Input|MouseEvents|MouseX
  (params (AxisValue :type Float%20%28single-precision%29))
  (bind _panspeed (Variables|CameraSetting|GetPanSpeed))
  (bind _ttscameraref (Variables|Reference|GetTTSCameraRef))
  (bind _returnvalue (Transformation|GetActorRotation _ttscameraref))
  (bind (_roll _pitch _yaw) (Math|Rotator|BreakRotator _returnvalue))
  ;[1 1 1] cam panning
  (Utilities|FlowControl|Gate true
    (:Exit
      (bind _output_get (Variables|Default|SetTimer (+ (Utilities|Time|GetWorldDeltaSeconds) (Variables|Default|GetTimer))))
      (if (>= _output_get 0.3)
        (Variables|Default|SetbIsPanning true)
        (Transformation|SetActorRotation (Variables|Reference|GetTTSCameraRef) (Math|Rotator|MakeRotator 0.0 (Math|Float|Clamp(Float) (+ _pitch (* _panspeed (stale Input|MouseEvents|MouseY AxisValue))) -3e+01 3e+01) (+ _yaw (* AxisValue _panspeed))))
        (else
          (Variables|Default|SetbIsPanning false))))))

(event Input|MouseEvents|MouseY
  (params (AxisValue :type Float%20%28single-precision%29))
  (bind _panspeed (Variables|CameraSetting|GetPanSpeed))
  (bind _ttscameraref (Variables|Reference|GetTTSCameraRef))
  (bind _returnvalue (Transformation|GetActorRotation _ttscameraref))
  (bind (_roll _pitch _yaw) (Math|Rotator|BreakRotator _returnvalue))
  ;[1 1 1] cam panning
  (Utilities|FlowControl|Gate true
    (:Exit
      (bind _output_get (Variables|Default|SetTimer (+ (Utilities|Time|GetWorldDeltaSeconds) (Variables|Default|GetTimer))))
      (if (>= _output_get 0.3)
        (Variables|Default|SetbIsPanning true)
        (Transformation|SetActorRotation (Variables|Reference|GetTTSCameraRef) (Math|Rotator|MakeRotator 0.0 (Math|Float|Clamp(Float) (+ _pitch (* _panspeed AxisValue)) -3e+01 3e+01) (+ _yaw (* (stale Input|MouseEvents|MouseX AxisValue) _panspeed))))
        (else
          (Variables|Default|SetbIsPanning false))))))

(event Input|MouseEvents|LeftMouseButton
  (params (Key :type Key%20Structure :default "None"))
  ;[1 1 1] player control select
  (:Pressed
    (CallFunction|ClearPiecefromSelection)
    (bind _asbp_ttspiece_base (Utilities|Casting|CastToBP_TTSPieceBase (.HitActor (Collision|BreakHitResult (.HitResult (Game|Player|GetHitResultUnderCursorbyChannel "TraceTypeQuery3" true)))))
      (:then
        (Variables|Reference|SetPieceSelection_Player _asbp_ttspiece_base)
        (CallFunction|AddPiecetoSelection _asbp_ttspiece_base))
      (:CastFailed
        (Variables|Reference|SetPieceSelection_Player _asbp_ttspiece_base)))))

(event Input|MouseEvents|RightMouseButton
  (params (Key :type Key%20Structure :default "None"))
  (bind _hitresult (Game|Player|GetHitResultUnderCursorbyChannel "TraceTypeQuery1" true))
  (bind _pieceselection_player (Variables|Reference|GetPieceSelection_Player))
  (bind (_bblockinghit _binitialoverlap _time _distance _location _impactpoint _normal _impactnormal _physmat _hitactor) (Collision|BreakHitResult _hitresult))
  ;[1 1 1] player control interact isn't control camera
  (:Released
    (if (not (== (Variables|Reference|GetPieceSelection_Player) (Variables|Default|GetNullActor)))
      (if (not (Variables|Default|GetbIsPanning))
        (bind _returnvalue (UserInterface|CreateWidget "/Game/BluePrint/HUD/WBP_TTSInterActMenuList.WBP_TTSInterActMenuList_C" (Game|GetPlayerController 0)))
        (bind _returnvalue_2 (Class|WidgetLayoutLibrary|GetMousePositiononViewport))
        (UserInterface|Viewport|AddtoViewport _returnvalue 0)
        (Class|UserWidget|SetPositioninViewport _returnvalue _returnvalue_2 true)
        (Variables|Default|SetMouseInteractPosition _location)
        (Variables|Default|SetInterActObjects _hitactor)
        (Variables|/Game/BluePrint/Piece/BP_TTSPieceBase.BP_TTSPieceBase_C|SetDesireLocation _pieceselection_player (Variables|Default|GetMouseInteractPosition))
        (Default|PieceInterAct (Variables|/Game/BluePrint/Piece/BP_TTSPieceBase.BP_TTSPieceBase_C|GetPieceActComponent _pieceselection_player) (Variables|Default|GetActionWhat))))))

(fn ConstructionScript)

(fn AddPiecetoSelection
  (params (Piece :type BP%20TTS%20Piece%20Base%20Object%20Reference))
  (Utilities|Array|AddUnique (Variables|Reference|GetSelection) Piece)
  (Default|IsPieceSelected Piece true))

(fn RemovePiecefromSelection
  (params (Piece :type BP%20TTS%20Piece%20Base%20Object%20Reference))
  (Utilities|Array|RemoveItem (Variables|Reference|GetSelection) Piece)
  (Default|IsPieceSelected Piece false))

(fn ClearPiecefromSelection
  (bind _selection (Variables|Reference|GetSelection))
  (for _array_element _selection
    (bind _asbp_ttspiece_base (Utilities|Casting|CastToBP_TTSPieceBase _array_element))
    (Default|IsPieceSelected _asbp_ttspiece_base false))
  (Utilities|Array|Clear _selection))