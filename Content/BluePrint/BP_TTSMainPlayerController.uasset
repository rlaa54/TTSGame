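; Player controller that drives the BP_TTSCameraPawn camera with movement, panning and zoom.
; BeginPlay caches the controlled pawn and its default spring arm length for zoom reset.
; MoveForward and MoveRight share one swept, horizontal location update along the camera's forward and right vectors.
; Holding Pan opens a gate for mouse-driven yaw and clamped pitch, while zoom steps the arm length within limits; both have resets.
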(event EventBeginPlay
  (Utilities|FlowControl|Sequence
    (:then_0
      (Utilities|ReferenceCast)
      (Variables|CameraSetting|SetZoomDefault (Variables|/Script/Engine.SpringArmComponent|GetTargetArmLength (Variables|/Game/BluePrint/BP_TTSCameraPawn.BP_TTSCameraPawn_C|GetSpringArm (Variables|Reference|GetTTSCameraRef)))))))

(event Input|ActionEvents|InputActionZoomIn
  (params (Key :type Key%20Structure :default "None"))
  (bind _ttscameraref (Variables|Reference|GetTTSCameraRef))
  (bind _springarm (Variables|/Game/BluePrint/BP_TTSCameraPawn.BP_TTSCameraPawn_C|GetSpringArm _ttscameraref))
  (:Pressed
    (Variables|/Script/Engine.SpringArmComponent|SetTargetArmLength _springarm (Math|Float|Clamp(Float) (- (Variables|/Script/Engine.SpringArmComponent|GetTargetArmLength _springarm) (Variables|CameraSetting|GetZoomSpeed)) (Variables|CameraSetting|GetZoomInMax) (Variables|CameraSetting|GetZoomOutMax)))))

(event Input|ActionEvents|InputActionZoomOut
  (params (Key :type Key%20Structure :default "None"))
  (bind _ttscameraref (Variables|Reference|GetTTSCameraRef))
  (bind _springarm (Variables|/Game/BluePrint/BP_TTSCameraPawn.BP_TTSCameraPawn_C|GetSpringArm _ttscameraref))
  (:Pressed
    (Variables|/Script/Engine.SpringArmComponent|SetTargetArmLength _springarm (Math|Float|Clamp(Float) (+ (Variables|CameraSetting|GetZoomSpeed) (Variables|/Script/Engine.SpringArmComponent|GetTargetArmLength _springarm)) (Variables|CameraSetting|GetZoomInMax) (Variables|CameraSetting|GetZoomOutMax)))))

(event Input|ActionEvents|InputActionZoomReset
  (params (Key :type Key%20Structure :default "None"))
  (:Pressed
    (Variables|/Script/Engine.SpringArmComponent|SetTargetArmLength (Variables|/Game/BluePrint/BP_TTSCameraPawn.BP_TTSCameraPawn_C|GetSpringArm (Variables|Reference|GetTTSCameraRef)) (Variables|CameraSetting|GetZoomDefault))))

(event Input|ActionEvents|InputActionPan
  (params (Key :type Key%20Structure :default "None"))
  (bind _panspeed (Variables|CameraSetting|GetPanSpeed))
  (bind _ttscameraref (Variables|Reference|GetTTSCameraRef))
  (bind _returnvalue (Transformation|GetActorRotation _ttscameraref))
  (bind (_roll _pitch _yaw) (Math|Rotator|BreakRotator _returnvalue))
  (:Pressed
    (Utilities|FlowControl|Gate true) ; enters at Open
  )
  (:Released
    (Utilities|FlowControl|Gate true) ; enters at Close
  ))

(event Input|ActionEvents|InputActionPanReset
  (params (Key :type Key%20Structure :default "None"))
  (:Pressed
    (Transformation|SetActorRotation (Variables|Reference|GetTTSCameraRef) (Math|Rotator|MakeRotator 0.0 0.0 0.0))))

(event Input|AxisEvents|InputAxisMoveForward
  (params (AxisValue :type Float%20%28single-precision%29))
  (bind _ttscameraref (Variables|Reference|GetTTSCameraRef))
  (bind _returnvalue (Transformation|GetActorForwardVector _ttscameraref))
  (bind _returnvalue_2 (Transformation|GetActorRightVector _ttscameraref))
  (bind (_x _y) (Math|Vector|BreakVector _returnvalue))
  (bind (_x_2 _y_2) (Math|Vector|BreakVector _returnvalue_2))
  (Transformation|SetActorLocation _ttscameraref (+ (Transformation|GetActorLocation _ttscameraref) (* (Math|Vector|MakeVector _x _y 0.0) (* AxisValue (Variables|CameraSetting|GetCameraSpeed))) (* (Math|Vector|MakeVector _x_2 _y_2 0.0) (* (stale Input|AxisEvents|InputAxisMoveRight AxisValue) (Variables|CameraSetting|GetCameraSpeed)))) true false))

(event Input|AxisEvents|InputAxisMoveRight
  (params (AxisValue :type Float%20%28single-precision%29))
  (bind _ttscameraref (Variables|Reference|GetTTSCameraRef))
  (bind _returnvalue (Transformation|GetActorForwardVector _ttscameraref))
  (bind _returnvalue_2 (Transformation|GetActorRightVector _ttscameraref))
  (bind (_x _y) (Math|Vector|BreakVector _returnvalue))
  (bind (_x_2 _y_2) (Math|Vector|BreakVector _returnvalue_2))
  (Transformation|SetActorLocation _ttscameraref (+ (Transformation|GetActorLocation _ttscameraref) (* (Math|Vector|MakeVector _x _y 0.0) (* (stale Input|AxisEvents|InputAxisMoveForward AxisValue) (Variables|CameraSetting|GetCameraSpeed))) (* (Math|Vector|MakeVector _x_2 _y_2 0.0) (* AxisValue (Variables|CameraSetting|GetCameraSpeed)))) true false))

(event Input|MouseEvents|MouseX
  (params (AxisValue :type Float%20%28single-precision%29))
  (bind _panspeed (Variables|CameraSetting|GetPanSpeed))
  (bind _ttscameraref (Variables|Reference|GetTTSCameraRef))
  (bind _returnvalue (Transformation|GetActorRotation _ttscameraref))
  (bind (_roll _pitch _yaw) (Math|Rotator|BreakRotator _returnvalue))
  (Utilities|FlowControl|Gate true
    (:Exit
      (Transformation|SetActorRotation (Variables|Reference|GetTTSCameraRef) (Math|Rotator|MakeRotator 0.0 (Math|Float|Clamp(Float) (+ _pitch (* _panspeed (stale Input|MouseEvents|MouseY AxisValue))) -4e+01 4e+01) (+ _yaw (* AxisValue _panspeed)))))))

(event Input|MouseEvents|MouseY
  (params (AxisValue :type Float%20%28single-precision%29))
  (bind _panspeed (Variables|CameraSetting|GetPanSpeed))
  (bind _ttscameraref (Variables|Reference|GetTTSCameraRef))
  (bind _returnvalue (Transformation|GetActorRotation _ttscameraref))
  (bind (_roll _pitch _yaw) (Math|Rotator|BreakRotator _returnvalue))
  (Utilities|FlowControl|Gate true
    (:Exit
      (Transformation|SetActorRotation (Variables|Reference|GetTTSCameraRef) (Math|Rotator|MakeRotator 0.0 (Math|Float|Clamp(Float) (+ _pitch (* _panspeed AxisValue)) -4e+01 4e+01) (+ _yaw (* (stale Input|MouseEvents|MouseX AxisValue) _panspeed)))))))

(fn ConstructionScript)