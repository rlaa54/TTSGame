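; HUD for the TTS canvas that pops up an interaction menu list widget at the mouse position.
; BeginPlay caches the local BP_TTSMainPlayerController as the owner for created widgets.
; ShowWidgetmouseposition creates a WBP_TTSInterActMenuList, removes and clears any menu held in InterActMenuBoxList, then places the new one at the cursor.
; The new widget is never stored in InterActMenuBoxList here.
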(event EventBeginPlay
  (bind _asbp_ttsmain_player_controller (Utilities|Casting|CastToBP_TTSMainPlayerController (Game|GetPlayerController 0)))
  (Variables|Default|SetPlayerControllerRef _asbp_ttsmain_player_controller))

(fn ConstructionScript)

(fn ShowWidgetmouseposition
  (bind _returnvalue (UserInterface|CreateWidget "/Game/BluePrint/HUD/WBP_TTSInterActMenuList.WBP_TTSInterActMenuList_C" (Variables|Default|GetPlayerControllerRef)))
  (Utilities|IsValid (Variables|Default|GetInterActMenuBoxList)
    (:Is%20Valid
      (Widget|RemovefromParent (Variables|Default|GetInterActMenuBoxList)))
    (:Is%20Not%20Valid
      _))
  (Variables|Default|SetInterActMenuBoxList 0)
  (bind _returnvalue_2 (Class|WidgetLayoutLibrary|GetMousePositiononViewport))
  (UserInterface|Viewport|AddtoViewport _returnvalue 0)
  (Class|UserWidget|SetPositioninViewport _returnvalue _returnvalue_2 false))