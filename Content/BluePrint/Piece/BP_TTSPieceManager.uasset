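; BP_TTSPieceManager caches every BP_TTSPieceBase actor at BeginPlay and builds a tree of piece interactions.
; StringTableInteraction parses each entry of the string table behind the "attack" text into name and parent structs by splitting on commas and colons.
; MakingInteractTree indexes them by name, then stores a flat array of nodes, each pairing an interaction with its looked-up parent.
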(event EventBeginPlay
  ;[1 1 1] when begin, get all actors of pieces and make interact tree
  (bind _outactors (Actor|GetAllActorsOfClass "/Game/BluePrint/Piece/BP_TTSPieceBase.BP_TTSPieceBase_C"))
  (Variables|Default|SetAllPiece _outactors)
  (for _array_element _outactors
    _)
  (CallFunction|MakingInteractTree))

(fn ConstructionScript)

(fn StringTableInteraction
  (bind _outtableid (Class|KismetTextLibrary|StringTableIdandKeyfromText "attack"))
  (for _array_element (Class|KismetStringTableLibrary|GetKeysfromStringTable _outtableid)
    (bind _output_get (Variables|Default|SetsInterAct (Utilities|Struct|MakeS_InterAct (.RightS (Utilities|String|Split (.RightS (Utilities|String|Split (Class|KismetStringTableLibrary|GetTableEntrySourceString _outtableid _array_element) ",")) ":")) (.RightS (Utilities|String|Split (.LeftS (Utilities|String|Split (Class|KismetStringTableLibrary|GetTableEntrySourceString _outtableid _array_element) ",")) ":")))))
    (Utilities|Array|Add (Variables|Default|GetsInterActArr) _output_get))
  (return (Variables|Default|GetsInterActArr)))

(fn MakingInteractTree
  (bind _sinteractdict (Variables|Default|GetsInteractDict))
  (bind _sinteract (CallFunction|StringTableInteraction))
  (for _array_element _sinteract
    (Utilities|Map|Add (Variables|Default|GetsInteractDict) (.NameStr (Utilities|Struct|BreakS_InterAct _array_element)) _array_element))
  (bind _values (Utilities|Map|Values _sinteractdict))
  (for _array_element_2 _values
    (Utilities|Array|Add (Variables|Default|GetsInteractNodeArr) (Utilities|Struct|MakeS_interactNode _array_element_2 (.Value (Utilities|Map|Find _sinteractdict (.Parent (Utilities|Struct|BreakS_InterAct _array_element_2))))))))