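; Base actor for a selectable game piece with a team, action points and turn requests to the game mode.
; Left-click toggles selection through the player controller using decal visibility as selected state, and hover drives a material highlight parameter.
; PieceInteract dispatches move, attack, activate or deactivate to PieceActComponent, then calls UsingActionPoint, which only deducts a point for moves.
; TurnRequesting passes the piece to the game mode when it is active.
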(event Custom|TurnRequesting
  ;[1 1 1] If piece activate then turn requset
  (if (Variables|Default|GetIsActivate)
    (bind _asbp_ttsgame_mode (Utilities|Casting|CastToBP_TTSGameMode (Game|GetGameMode)))
    (Default|TurnRequest _asbp_ttsgame_mode self)))

(event MouseInput|EventActorBeginCursorOver
  ;[1 1 1] when piece selected then highlight
  (Variables|Default|SetPieceHighlighted 1.0)
  (Rendering|Material|SetScalarParameterValueonMaterials (Variables|Character|GetMesh) "Highlighted" (Variables|Default|GetPieceHighlighted)))

(event MouseInput|EventActorOnClicked
  (params (ButtonPressed :type Key%20Structure :default "None"))
  (bind _self self)
  (bind _ttsplayercontrollerref (Variables|Default|GetTTSPlayerControllerRef))
  ;[1 1 1] Piece mouse click then select
  (if (== ButtonPressed "LeftMouseButton")
    (if (Rendering|IsVisible (Variables|Default|GetDecal))
      (Default|RemovePiecefromSelection _ttsplayercontrollerref _self)
      (else
        (Default|AddPiecetoSelection _ttsplayercontrollerref _self)))))

(event MouseInput|EventActorEndCursorOver
  ;[1 1 1] when piece selected then highlight
  (Variables|Default|SetPieceHighlighted 0.0)
  (Rendering|Material|SetScalarParameterValueonMaterials (Variables|Character|GetMesh) "Highlighted" (Variables|Default|GetPieceHighlighted)))

(event EventBeginPlay
  ;[1 1 1] piece init
  (bind _asbp_ttsmain_player_controller (Utilities|Casting|CastToBP_TTSMainPlayerController (Game|GetPlayerController 0)))
  (Variables|Default|SetTTSPlayerControllerRef _asbp_ttsmain_player_controller)
  (Variables|Default|SetCurrentActionPoint (Variables|Default|GetMaxActionPoint))
  (Variables|Default|SetTeam 1))

(fn ConstructionScript)

(fn IsPieceSelected
  (params (IsSelected :type Boolean))
  (Variables|Default|SetbIsSelected IsSelected)
  (Rendering|SetVisibility (Variables|Default|GetDecal) IsSelected false))

(fn PieceInteract
  (bind _pieceactcomponent (Variables|Default|GetPieceActComponent))
  (switch Utilities|FlowControl|Switch|SwitchonE_InterAct (Variables|Default|GeteInterAct)
    (:NewEnumerator0
      (Default|Move _pieceactcomponent))
    (:NewEnumerator1
      (Default|Attack _pieceactcomponent))
    (:NewEnumerator2
      (Default|Active _pieceactcomponent))
    (:NewEnumerator3
      (Default|Deactive _pieceactcomponent)))
  (CallFunction|UsingActionPoint))

(fn UsingActionPoint
  (bind _self self)
  (switch Utilities|FlowControl|Switch|SwitchonE_InterAct (Variables|Default|GeteInterAct)
    (:NewEnumerator0
      (Variables|BP_TTSPieceBase_C|SetCurrentActionPoint _self (- (Variables|BP_TTSPieceBase_C|GetCurrentActionPoint _self) 1)))))